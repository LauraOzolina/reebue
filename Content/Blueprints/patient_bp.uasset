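; Patient actor Blueprint that can be nudged vertically and along the X axis, as if on an adjustable bed.
; Four functions (LiftPatient, LowerPatient, MoveBedIn, MoveBedOut) each offset the actor's location by one world-space unit per call, without sweep or limits.
; The event graph and construction script are empty, so movement happens only when these functions are called.
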(event EventBeginPlay)

(event Collision|EventActorBeginOverlap
  (params (OtherActor :type Actor%20Object%20Reference)))

(event EventTick
  (params (DeltaSeconds :type Float%20%28single-precision%29)))

(fn ConstructionScript)

(fn LiftPatient
  (Transformation|SetActorLocation (+ (Transformation|GetActorLocation) "0,0,1.000000") false false))

(fn LowerPatient
  (Transformation|SetActorLocation (+ (Transformation|GetActorLocation) "0,0,-1.000000") false false))

(fn MoveBedin
  (Transformation|SetActorLocation (+ (Transformation|GetActorLocation) "-1.000000,0,0.000000") false false))

(fn MoveBedOut
  (Transformation|SetActorLocation (+ (Transformation|GetActorLocation) "1.000000,0,0.000000") false false))